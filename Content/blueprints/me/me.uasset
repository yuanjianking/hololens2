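; The "me" player actor acts as a push-to-talk voice source that can alert AI.
; Holding Space records the microphone through AudioCapture and submix output recording; releasing plays the clip back in 2D and reports a noise event tagged "me" at the actor's location.
; A separate Timerhandler flags a timeout and resets the AI controller's blackboard.
; The camera-follow movement is disconnected, so Tick does nothing.
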(event EventTick
  (params (DeltaSeconds :type Float%20%28single-precision%29))
  ;[1 1 1] 跟随相机移动玩家自身位置
)

(event Input|KeyboardEvents|SpaceBar
  (params (Key :type Key%20Structure :default "None"))
  (bind _audiocapture (Variables|Default|GetAudioCapture))
  ;[1 1 1] 开启录音
  (:Pressed
    (bind _outdevices (Class|MediaBlueprintFunctionLibrary|EnumerateAudioCaptureDevices -1))
    (if (>= (Utilities|Array|Length _outdevices) 1)
      (Components|Activation|SetActive _audiocapture true true)
      (Audio|Components|Audio|SetVolumeMultiplier _audiocapture 0.5 :!class /Script/AudioMixer.SynthComponent)
      (CameraShake|Start _audiocapture)
      (Class|AudioMixerBlueprintLibrary|StartRecordingOutput 0.0 0)
      (else
        (Development|PrintString "no audio device"))))
  (:Released
    (bind _returnvalue (Class|AudioMixerBlueprintLibrary|StopRecordingOutput "SoundWave" "test" "" 0 0))
    (Audio|PlaySound2D _returnvalue 1.0 1.0 0.0 0 0)
    (Audio|Components|Audio|Stop (Variables|Default|GetAudioCapture))
    (Class|AISenseHearing|ReportNoiseEvent (Transformation|GetActorLocation) 1.0 self 0.0 "me")))

(fn ConstructionScript)

(fn Timerhandler
  ;[1 1 1] 更新NPC状态
  (Variables|Default|SetisTimeOut true)
  (Default|RestBlackBoard (Variables|Default|GetAiContorller)))